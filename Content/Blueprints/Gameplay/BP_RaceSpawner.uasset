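; BP_RaceSpawner is a race spawner actor that creates a player and vehicle for each entry in the game instance's vehicle list.
; On BeginPlay it creates local players beyond the first and spawns each vehicle class at its own transform with a player ID and numbered racer name.
; Each pass also destroys a BP_CustomArcadeVehicle found before spawning, then has the matching player controller possess the new vehicle.
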(event `self.ReceiveBeginPlay`
  (bind _asgi_custom_vehicle_game_instance (cast `/Game/Blueprints/GI_CustomVehicleGameInstance` (`GameplayStatics.GetGameInstance`)))
  (for (_array_element _array_index) (`/Game/Blueprints/GI_CustomVehicleGameInstance.vehicles` _asgi_custom_vehicle_game_instance)
    (`KismetSystemLibrary.PrintString` (`KismetSystemLibrary.GetClassDisplayName` _array_element))
    (if (> _array_index 0)
      (`GameplayStatics.CreatePlayer` _array_index))
    (bind _returnvalue (`GameplayStatics.GetActorOfClass` "/Game/Blueprints/Cars/CustomArcadeVehicle/BP_CustomArcadeVehicle.BP_CustomArcadeVehicle_C"))
    (bind _returnvalue_2 (`|SpawnActorFromClass` _array_element (`self.GetTransform`) "Undefined" "OverrideRootScale" null _array_index (`KismetTextLibrary.Conv_StringToText` (`KismetStringLibrary.Concat_StrStr` "Racer " (`KismetStringLibrary.Conv_IntToString` (+ _array_index 1)))) null))
    (`self.K2_DestroyActor` _returnvalue)
    (bind _returnvalue_3 (`GameplayStatics.GetPlayerControllerFromID` _array_index))
    (`Controller.UnPossess` _returnvalue_3)
    (`Controller.Possess` _returnvalue_3 _returnvalue_2)))

(fn `UserConstructionScript`)