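; BP_Item is a spinning pickup cube that can give a BP_CustomArcadeVehicle a random item.
; On overlap with that vehicle, PickItem hides the cube, disables its collision and starts a timer that calls RespawnItem ten seconds later.
; The vehicle's CurrentItemType changes only if it equals one specific enum value.
; The random pick from ItemTypes never selects the last entry, as RandomInteger receives Length minus one.
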(event `self.ReceiveTick`
  (params (DeltaSeconds :type "Float (single-precision)"))
  (bind _returnvalue (* DeltaSeconds (`self.rotationSpeed`)))
  (`SceneComponent.K2_AddLocalRotation` (`self.Cube`) (`KismetMathLibrary.MakeRotator` (* _returnvalue -1.0) _returnvalue _returnvalue) false false))

(event `self.Cube.OnComponentBeginOverlap`
  (params (OverlappedComponent :type "PrimitiveComponent Object Reference") (OtherActor :type "Actor Object Reference") (OtherComp :type "PrimitiveComponent Object Reference") (OtherBodyIndex :type Integer) (bFromSweep :type Boolean) (SweepResult :type "HitResult Structure (by ref)"))
  (bind _itemtypes (`self.itemTypes`))
  (bind _asbp_custom_arcade_vehicle (cast `/Game/Blueprints/Cars/CustomArcadeVehicle/BP_CustomArcadeVehicle` OtherActor))
  (`self.PickItem`)
  (if (`|EnumEquality` (`/Game/Blueprints/Cars/CustomArcadeVehicle/BP_CustomArcadeVehicle.currentItemType` _asbp_custom_arcade_vehicle) "NewEnumerator2")
    (set `/Game/Blueprints/Cars/CustomArcadeVehicle/BP_CustomArcadeVehicle.currentItemType` (`|GetArrayItem` _itemtypes (`KismetMathLibrary.RandomInteger` (- (`KismetArrayLibrary.Array_Length` _itemtypes) 1))) _asbp_custom_arcade_vehicle)))

(fn `PickItem`
  (bind _cube (`self.Cube`))
  (`PrimitiveComponent.SetCollisionEnabled` _cube "NoCollision")
  (`SceneComponent.SetHiddenInGame` _cube true false)
  (`KismetSystemLibrary.K2_SetTimer` self "RespawnItem" 10.0))

(fn `RespawnItem`
  (bind _cube (`self.Cube`))
  (`PrimitiveComponent.SetCollisionEnabled` _cube "QueryAndPhysics")
  (`SceneComponent.SetHiddenInGame` _cube false false))

(fn `UserConstructionScript`)