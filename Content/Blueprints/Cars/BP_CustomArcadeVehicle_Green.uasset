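; Green variant of the custom arcade vehicle, built as a child Blueprint on inherited setup and suspension logic.
; On BeginPlay it runs the parent logic, then sets its own suspension height.
; Any damage briefly freezes physics on the vehicle's collision, then re-enables it after a short delay and replays the suspension init timeline from the start.
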(event `self.ReceiveBeginPlay`
  (`parent.ReceiveBeginPlay`)
  (set `self.suspensionHeight` 20.0))

(event `self.ReceiveAnyDamage`
  (params (Damage :type "Float (single-precision)") (DamageType :type "DamageType Object Reference") (InstigatedBy :type "Controller Object Reference") (DamageCauser :type "Actor Object Reference"))
  ;[1 0.8557 0] Get Damage
  (`PrimitiveComponent.SetSimulatePhysics` (`self.VehicleCollision`) false)
  (`KismetSystemLibrary.Delay` 0.3)
  (`PrimitiveComponent.SetSimulatePhysics` (`self.VehicleCollision`) true)
  (`TimelineComponent.PlayFromStart` (`self.SuspensionInitTimeline`)))

(fn `UserConstructionScript`
  (`parent.UserConstructionScript`))