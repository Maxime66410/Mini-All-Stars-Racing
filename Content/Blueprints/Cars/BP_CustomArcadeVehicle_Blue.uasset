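; Blue arcade vehicle Blueprint that extends a parent vehicle with an animated lever and a damage reaction.
; Each tick, the rounded steering axis selects one of three roll targets, and the lever interpolates toward it.
; Any damage briefly disables collision-body physics simulation and swaps the skeletal mesh to a hit material.
; After a short delay, both are restored and the suspension init timeline replays from the start.
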(event `self.ReceiveTick`
  (params (DeltaSeconds :type "Float (single-precision)"))
  (`parent.ReceiveTick` DeltaSeconds)
  (`self.Lever Rotation`))

(event `Lever Rotation`
  (bind _lever (`self.Lever`))
  (bind (_returnvalue_location _returnvalue_rotation) (`KismetMathLibrary.BreakTransform` (`SceneComponent.GetRelativeTransform` _lever)))
  ;[1 0.278 0.8336] Lever rotation
  (bind _output_get (set `self.Direction` (`KismetMathLibrary.Round` (`self.currentSteeringAxis`))))
  (switch `int` _output_get
    (:`-1`
      (set `self.Target X (Roll)` -90.0))
    (:`0`
      (set `self.Target X (Roll)` -40.0))
    (:`1`
      (set `self.Target X (Roll)` 0.0)))
  (`SceneComponent.K2_SetRelativeRotation` _lever (`KismetMathLibrary.RInterpTo` _returnvalue_rotation (`KismetMathLibrary.MakeRotator` (`self.Target X (Roll)`) 90.0) (`self.deltaSeconds`) 1.0) false false))

(event `self.ReceiveAnyDamage`
  (params (Damage :type "Float (single-precision)") (DamageType :type "DamageType Object Reference") (InstigatedBy :type "Controller Object Reference") (DamageCauser :type "Actor Object Reference"))
  (bind _skeletalmesh (`self.SkeletalMesh`))
  ;[1 0.8557 0] Get Damage
  (`PrimitiveComponent.SetSimulatePhysics` (`self.VehicleCollision`) false)
  (`PrimitiveComponent.SetMaterial` _skeletalmesh 0 "/Game/Assets/Personnage/Steve/M_SteveDiffuseHit.M_SteveDiffuseHit")
  (`KismetSystemLibrary.Delay` 0.3)
  (`PrimitiveComponent.SetMaterial` _skeletalmesh 0 "/Game/Assets/Personnage/Steve/M_SteveDiffuse.M_SteveDiffuse")
  (`PrimitiveComponent.SetSimulatePhysics` (`self.VehicleCollision`) true)
  (`TimelineComponent.PlayFromStart` (`self.SuspensionInitTimeline`)))

(fn `UserConstructionScript`
  (`parent.UserConstructionScript`))