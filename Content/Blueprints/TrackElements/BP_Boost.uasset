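; BP_Boost is a track element that gives a speed boost to arcade vehicles that drive into it.
; When its Box is overlapped, it casts to the player vehicle, then the AI vehicle, and calls SpeedBoostStart with configurable strength, duration and auto-stop.
; It also plays a sound assigned at BeginPlay and sets an action state on the boosted vehicle.
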(event `self.ReceiveBeginPlay`
  (`AudioComponent.SetSound` (`self.Audio`) (`self.Sound`)))

(event `self.Box.OnComponentBeginOverlap`
  (params (OverlappedComponent :type "PrimitiveComponent Object Reference") (OtherActor :type "Actor Object Reference") (OtherComp :type "PrimitiveComponent Object Reference") (OtherBodyIndex :type Integer) (bFromSweep :type Boolean) (SweepResult :type "HitResult Structure (by ref)"))
  (bind _asbp_custom_arcade_vehicle (cast `/Game/Blueprints/Cars/CustomArcadeVehicle/BP_CustomArcadeVehicle` OtherActor)
    (:`then`
      (`/Game/Blueprints/Cars/CustomArcadeVehicle/BP_CustomArcadeVehicle.SpeedBoostStart` _asbp_custom_arcade_vehicle (`self.boostValue`) (`self.autoStopBoost`) (`self.boostTime`))
      (`AudioComponent.Play` (`self.Audio`) 0.0)
      (`/Game/Blueprints/Cars/CustomArcadeVehicle/BP_CustomArcadeVehicle.SetActionsPlayer` _asbp_custom_arcade_vehicle "NewEnumerator2"))
    (:`CastFailed`
      (bind _asbp_custom_arcade_vehicle_ai (cast `/Game/Assets/Blueprint/AI/BP_CustomArcadeVehicle_AI` OtherActor))
      (`/Game/Assets/Blueprint/AI/BP_CustomArcadeVehicle_AI.SpeedBoostStart` _asbp_custom_arcade_vehicle_ai (`self.boostValue`) (`self.autoStopBoost`) (`self.boostTime`))
      (`AudioComponent.Play` (`self.Audio`) 0.0)
      (`/Game/Assets/Blueprint/AI/BP_CustomArcadeVehicle_AI.SetActionsPlayer` _asbp_custom_arcade_vehicle_ai "NewEnumerator2"))))

(fn `UserConstructionScript`)