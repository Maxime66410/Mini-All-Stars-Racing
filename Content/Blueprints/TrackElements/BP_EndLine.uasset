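; Finish line that counts laps, times the race and records standings for player and AI arcade vehicles.
; GoodSideEntry flags correct-direction entries and makes Box passable, with collision settings reapplied every Tick.
; Box overlaps update player lap and respawn point, or unpossess finishers; the AI lap update receives no vehicle.
; Players get an end-race widget, and the main menu loads after a delay once standings match the BP_CustomArcadeVehicle count.
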(event `self.ReceiveBeginPlay`
  (bind _returnvalue (`|CreateWidget` "/Game/UI/WBP_Timer.WBP_Timer_C" null self))
  (`UserWidget.AddToPlayerScreen` _returnvalue 0)
  (`AudioComponent.SetSound` (`self.Audio`) (`self.Sound`)))

(event `self.ReceiveTick`
  (params (DeltaSeconds :type "Float (single-precision)"))
  (`self.ManageCollisions`)
  (if (`self.shouldUpdateTimer`)
    (set `self.timer` (+ (`self.timer`) DeltaSeconds))))

(event `self.Box.OnComponentBeginOverlap`
  (params (OverlappedComponent :type "PrimitiveComponent Object Reference") (OtherActor :type "Actor Object Reference") (OtherComp :type "PrimitiveComponent Object Reference") (OtherBodyIndex :type Integer) (bFromSweep :type Boolean) (SweepResult :type "HitResult Structure (by ref)"))
  (bind _asbp_custom_arcade_vehicle (cast `/Game/Blueprints/Cars/CustomArcadeVehicle/BP_CustomArcadeVehicle` OtherActor)
    (:`then`
      (if (`/Game/Blueprints/Cars/CustomArcadeVehicle/BP_CustomArcadeVehicle.isEnteringProperly` _asbp_custom_arcade_vehicle)
        (set `/Game/Blueprints/Cars/CustomArcadeVehicle/BP_CustomArcadeVehicle.isEnteringProperly` false _asbp_custom_arcade_vehicle)
        (if (>= (`/Game/Blueprints/Cars/CustomArcadeVehicle/BP_CustomArcadeVehicle.currentLoop` _asbp_custom_arcade_vehicle) (`self.loops`))
          (`KismetArrayLibrary.Array_Add` (`self.standings`) (make `/Game/Blueprints/Gameplay/S_standings` (`/Game/Blueprints/Cars/CustomArcadeVehicle/BP_CustomArcadeVehicle.playerName` _asbp_custom_arcade_vehicle) (`self.timer`)))
          (`Controller.UnPossess` (`Pawn.GetController` _asbp_custom_arcade_vehicle))
          (bind _returnvalue (`|CreateWidget` "/Game/UI/WBP_EndRace.WBP_EndRace_C" (`GameplayStatics.GetPlayerControllerFromID` (`/Game/Blueprints/Cars/CustomArcadeVehicle/BP_CustomArcadeVehicle.playerID` _asbp_custom_arcade_vehicle)) self))
          (`UserWidget.AddToPlayerScreen` _returnvalue 0)
          (`self.CheckEndRace`)
          (else
            (`self.UpdateRespawnPosition` _asbp_custom_arcade_vehicle)))))
    (:`CastFailed`
      (bind _asbp_custom_arcade_vehicle_ai (cast `/Game/Assets/Blueprint/AI/BP_CustomArcadeVehicle_AI` OtherActor))
      (if (`/Game/Assets/Blueprint/AI/BP_CustomArcadeVehicle_AI.isEnteringProperly` _asbp_custom_arcade_vehicle_ai)
        (set `/Game/Assets/Blueprint/AI/BP_CustomArcadeVehicle_AI.isEnteringProperly` false _asbp_custom_arcade_vehicle_ai)
        (if (>= (`/Game/Assets/Blueprint/AI/BP_CustomArcadeVehicle_AI.currentLoop` _asbp_custom_arcade_vehicle_ai) (`self.loops`))
          (`KismetArrayLibrary.Array_Add` (`self.standings`) (make `/Game/Blueprints/Gameplay/S_standings` (`/Game/Assets/Blueprint/AI/BP_CustomArcadeVehicle_AI.playerName` _asbp_custom_arcade_vehicle_ai) (`self.timer`)))
          (`Controller.UnPossess` (`Pawn.GetController` _asbp_custom_arcade_vehicle_ai))
          (else
            (`self.UpdateRespawnPosition` null)))))))

(event `self.Box.OnComponentEndOverlap`
  (params (OverlappedComponent :type "PrimitiveComponent Object Reference") (OtherActor :type "Actor Object Reference") (OtherComp :type "PrimitiveComponent Object Reference") (OtherBodyIndex :type Integer))
  (if (<= (`KismetArrayLibrary.Array_Length` (`PrimitiveComponent.GetOverlappingActors` (`self.goodSideEntry`) "/Game/Blueprints/Cars/CustomArcadeVehicle/BP_CustomArcadeVehicle.BP_CustomArcadeVehicle_C")) 0)
    (`self.UpdateCollisions` "QueryAndPhysics")
    (elif (<= (`KismetArrayLibrary.Array_Length` (`PrimitiveComponent.GetOverlappingActors` (`self.goodSideEntry`) "/Game/Assets/Blueprint/AI/BP_CustomArcadeVehicle_AI.BP_CustomArcadeVehicle_AI_C")) 0)
      (`self.UpdateCollisions` "QueryAndPhysics"))))

(event `self.goodSideEntry.OnComponentBeginOverlap`
  (params (OverlappedComponent :type "PrimitiveComponent Object Reference") (OtherActor :type "Actor Object Reference") (OtherComp :type "PrimitiveComponent Object Reference") (OtherBodyIndex :type Integer) (bFromSweep :type Boolean) (SweepResult :type "HitResult Structure (by ref)"))
  (bind _asbp_custom_arcade_vehicle (cast `/Game/Blueprints/Cars/CustomArcadeVehicle/BP_CustomArcadeVehicle` OtherActor)
    (:`then`
      (set `/Game/Blueprints/Cars/CustomArcadeVehicle/BP_CustomArcadeVehicle.isEnteringProperly` true _asbp_custom_arcade_vehicle)
      (`self.UpdateCollisions` "QueryOnly" "ECR_Overlap" "ECC_GameTraceChannel1"))
    (:`CastFailed`
      (bind _asbp_custom_arcade_vehicle_ai (cast `/Game/Assets/Blueprint/AI/BP_CustomArcadeVehicle_AI` OtherActor))
      (set `/Game/Assets/Blueprint/AI/BP_CustomArcadeVehicle_AI.isEnteringProperly` true _asbp_custom_arcade_vehicle_ai)
      (`self.UpdateCollisions` "QueryOnly" "ECR_Overlap" "ECC_GameTraceChannel1"))))

(fn `CheckEndRace`
  (bind _outactors (`GameplayStatics.GetAllActorsOfClass` "/Game/Blueprints/Cars/CustomArcadeVehicle/BP_CustomArcadeVehicle.BP_CustomArcadeVehicle_C"))
  (if (== (`KismetArrayLibrary.Array_Length` _outactors) (`KismetArrayLibrary.Array_Length` (`self.standings`)))
    (set `self.shouldUpdateTimer` false)
    (`KismetSystemLibrary.K2_SetTimer` null "LoadMainMenu" 5.0)))

(fn `LoadMainMenu`
  (`GameplayStatics.OpenLevel` "VehicleAdvExampleMap"))

(fn `ManageCollisions`
  (bind _box (`self.Box`))
  (`PrimitiveComponent.SetCollisionEnabled` _box (`self.collisionPreset`))
  (`PrimitiveComponent.SetCollisionResponseToChannel` _box "ECC_Vehicle" (`self.collisionResponseToVehicle`))
  (`PrimitiveComponent.SetCollisionObjectType` _box (`self.collisionObjectType`)))

(fn `UpdateCollisions`
  (params (Preset :type "ECollisionEnabled Enum" :default "QueryAndPhysics") (Response :type "ECollisionResponse Enum" :default "ECR_Block") (ObjectType :type "ECollisionChannel Enum" :default "ECC_WorldStatic"))
  (set `self.collisionPreset` Preset)
  (set `self.collisionResponseToVehicle` Response)
  (set `self.collisionObjectType` ObjectType))

(fn `UpdateRespawnPosition`
  (params (vehicle :type "/Game/Blueprints/Cars/CustomArcadeVehicle/BP_CustomArcadeVehicle Object Reference") (vehicleAI :type "/Game/Assets/Blueprint/AI/BP_CustomArcadeVehicle_AI Object Reference"))
  (`/Engine/EditorBlueprintResources/StandardMacros.IsValid` vehicle
    (:`Is Valid`
      (if (`/Game/Blueprints/Cars/CustomArcadeVehicle/BP_CustomArcadeVehicle.IsEntry?` vehicle)
        (set `/Game/Blueprints/Cars/CustomArcadeVehicle/BP_CustomArcadeVehicle.currentLoop` (+ (`/Game/Blueprints/Cars/CustomArcadeVehicle/BP_CustomArcadeVehicle.currentLoop` vehicle) 1) vehicle)
        (set `/Game/Blueprints/Cars/CustomArcadeVehicle/BP_CustomArcadeVehicle.lastCheckPointPosition` (`SceneComponent.K2_GetComponentToWorld` (`self.spawnPosition`)) vehicle)
        (set `/Game/Blueprints/Cars/CustomArcadeVehicle/BP_CustomArcadeVehicle.IsEntry?` false vehicle)
        (`AudioComponent.Play` (`self.Audio`) 0.0)))
    (:`Is Not Valid`
      (`/Engine/EditorBlueprintResources/StandardMacros.IsValid` vehicleAI
        (:`Is Valid`
          (if (`/Game/Assets/Blueprint/AI/BP_CustomArcadeVehicle_AI.IsEntry?` vehicleAI)
            (set `/Game/Assets/Blueprint/AI/BP_CustomArcadeVehicle_AI.currentLoop` (+ (`/Game/Assets/Blueprint/AI/BP_CustomArcadeVehicle_AI.currentLoop` vehicleAI) 1) vehicleAI)
            (set `/Game/Assets/Blueprint/AI/BP_CustomArcadeVehicle_AI.lastCheckPointPosition` (`SceneComponent.K2_GetComponentToWorld` (`self.spawnPosition`)) vehicleAI)
            (set `/Game/Assets/Blueprint/AI/BP_CustomArcadeVehicle_AI.IsEntry?` false vehicleAI)
            (`AudioComponent.Play` (`self.Audio`) 0.0)))))))

(fn `UserConstructionScript`)