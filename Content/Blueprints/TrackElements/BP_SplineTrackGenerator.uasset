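; Track element actor that builds a track along its spline from a configurable mesh and material.
; The construction script calls GenerateTrack, which divides the spline by a section length multiplied by actor X scale and adds one colliding spline mesh per section.
; Each segment takes its endpoints, tangents and roll from the spline, with tangents clamped to section length.
; The event graph is empty, so all work happens at construction.
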(fn `GenerateTrack`
  (params (staticMesh :type "StaticMesh Object Reference") (meshMaterial :type "MaterialInstance Object Reference") (scale :type "Vector Structure" :default (1.0 1.0 1.0)) (orientation :type "ESplineMeshAxis Enum" :default "X"))
  (bind _returnvalue_x (`KismetMathLibrary.BreakVector` (`self.GetActorScale3D`)))
  (bind _spline (`self.Spline`))
  (bind _sectionlength (`self.sectionLength`))
  (set `self.sectionLength` (* _returnvalue_x (`self.sectionLength`)))
  (for _index (range (+ (`KismetMathLibrary.FTrunc` (/ (`SplineComponent.GetSplineLength` (`self.Spline`)) (`self.sectionLength`))) 1))
    (bind _returnvalue (`AddComponent|NODE_AddSplineMeshComponent-1`))
    (`StaticMeshComponent.SetStaticMesh` _returnvalue staticMesh)
    (`PrimitiveComponent.SetMaterial` _returnvalue 0 meshMaterial)
    (`SplineMeshComponent.SetForwardAxis` _returnvalue orientation true)
    (`PrimitiveComponent.SetCollisionEnabled` _returnvalue "QueryAndPhysics")
    (`SceneComponent.SetRelativeScale3D` _returnvalue scale)
    (bind _returnvalue_2 (* _index _sectionlength))
    (bind _returnvalue_3 (* (+ _index 1) _sectionlength))
    (`SplineMeshComponent.SetStartAndEnd` _returnvalue (`SplineComponent.GetLocationAtDistanceAlongSpline` _spline _returnvalue_2 "Local") (`KismetMathLibrary.ClampVectorSize` (`SplineComponent.GetTangentAtDistanceAlongSpline` _spline _returnvalue_2 "Local") 0.0 (`self.sectionLength`)) (`SplineComponent.GetLocationAtDistanceAlongSpline` _spline _returnvalue_3 "Local") (`KismetMathLibrary.ClampVectorSize` (`SplineComponent.GetTangentAtDistanceAlongSpline` _spline _returnvalue_3 "Local") 0.0 (`self.sectionLength`)) true)
    (`SplineMeshComponent.SetStartRoll` _returnvalue (`KismetMathLibrary.DegreesToRadians` (`SplineComponent.GetRollAtDistanceAlongSpline` _spline _returnvalue_2 "Local")) true)
    (`SplineMeshComponent.SetEndRoll` _returnvalue (`KismetMathLibrary.DegreesToRadians` (`SplineComponent.GetRollAtDistanceAlongSpline` _spline _returnvalue_3 "Local")) true)))

(fn `UserConstructionScript`
  (`self.GenerateTrack` (`self.staticMesh`) (`self.meshMaterial`) (`self.meshScale`) (`self.meshOrientation`)))