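; BP_CarPicker is a per-player selector for choosing one of four colored vehicles before a multiplayer map loads.
; MoveRight cycles the slot with a timer-based cooldown, and Tick interpolates the picker's X toward the matching BP_PosCarPicker actor.
; MoveForward locks a car no other picker has locked, triggers its selection interaction and stores its class in the GameInstance by ControllerID.
; After a delay, it opens the GameInstance's map if every picker is locked.
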(event `self.ReceiveBeginPlay`
  (bind _asgi_custom_vehicle_game_instance (cast `/Game/Blueprints/GI_CustomVehicleGameInstance` (`GameplayStatics.GetGameInstance`)))
  (set `self.gameInstance` _asgi_custom_vehicle_game_instance)
  (`self.MakeArray`))

(event `InputAxis|MoveRight`
  (params (AxisValue :type "Float (single-precision)"))
  (if (and (!= AxisValue 0.0) (not (`self.carLocked`)) (not (`self.changingPos`)))
    (set `self.changingPos` true)
    (if (> AxisValue 0.0)
      (switch `int` (`self.carPosition`)
        (:`0`
          (set `self.carPosition` 1))
        (:`1`
          (set `self.carPosition` 2))
        (:`2`
          (set `self.carPosition` 3))
        (:`3`
          (set `self.carPosition` 0)))
      (`KismetSystemLibrary.K2_SetTimer` null "HoveredCarChanged" 0.2 :!label _label)
      (elif (< AxisValue 0.0)
        (switch `int` (`self.carPosition`)
          (:`0`
            (set `self.carPosition` 3)
            (goto _label))
          (:`1`
            (set `self.carPosition` 0)
            (goto _label))
          (:`2`
            (set `self.carPosition` 1)
            (goto _label))
          (:`3`
            (set `self.carPosition` 2)
            (goto _label)))))))

(event `InputAxis|MoveForward`
  (params (AxisValue :type "Float (single-precision)"))
  (bind _vehiclechosen (`self.vehicleChosen`))
  (if (> AxisValue 0.0)
    (set `self.canLock` true)
    (bind _outactors (`GameplayStatics.GetAllActorsOfClass` "BP_CarPicker_C"))
    (for _array_element _outactors
      (if (and (!= _array_element self) (`/Game/Blueprints/BP_CarPicker.carLocked` _array_element) (== (`/Game/Blueprints/BP_CarPicker.carPosition` _array_element) (`self.carPosition`)))
        (set `self.canLock` false)))
    (if (`self.canLock`)
      (set `self.carLocked` true)
      (switch `int` (`self.carPosition`)
        (:`0`
          (bind _returnvalue (`GameplayStatics.GetActorOfClass` "/Game/Blueprints/Cars/BP_CustomArcadeVehicle_Blue.BP_CustomArcadeVehicle_Blue_C"))
          (set `self.vehicleChosen` _returnvalue))
        (:`1`
          (bind _returnvalue_2 (`GameplayStatics.GetActorOfClass` "/Game/Blueprints/Cars/BP_CustomArcadeVehicle_Green.BP_CustomArcadeVehicle_Green_C"))
          (set `self.vehicleChosen` _returnvalue_2))
        (:`2`
          (bind _returnvalue_3 (`GameplayStatics.GetActorOfClass` "/Game/Blueprints/Cars/BP_CustomArcadeVehicle_Red.BP_CustomArcadeVehicle_Red_C"))
          (set `self.vehicleChosen` _returnvalue_3))
        (:`3`
          (bind _returnvalue_4 (`GameplayStatics.GetActorOfClass` "/Game/Blueprints/Cars/BP_CustomArcadeVehicle_Yellow.BP_CustomArcadeVehicle_Yellow_C"))
          (set `self.vehicleChosen` _returnvalue_4)))
      (`/Game/Blueprints/Cars/CustomArcadeVehicle/BP_CustomArcadeVehicle.SelectCarInteraction` _vehiclechosen)
      (`KismetArrayLibrary.Array_Set` (`/Game/Blueprints/GI_CustomVehicleGameInstance.vehicles` (`self.gameInstance`)) (`self.controllerID`) (`GameplayStatics.GetObjectClass` _vehiclechosen))
      (`KismetSystemLibrary.Delay` 1.0)
      (`self.CheckIfAllPlayersAreReady`))))

(event `self.ReceiveTick`
  (params (DeltaSeconds :type "Float (single-precision)"))
  (set `self.Delta Seconds` DeltaSeconds)
  (`self.UpdatePickerPosition`))

(fn `CheckIfAllPlayersAreReady`
  (locals (canLaunchMap :type Boolean))
  (set `local.canLaunchMap` true)
  (bind _outactors (`GameplayStatics.GetAllActorsOfClass` "BP_CarPicker_C"))
  (for _array_element _outactors
    (if (not (`/Game/Blueprints/BP_CarPicker.carLocked` _array_element))
      (set `local.canLaunchMap` false)))
  (if (`local.canLaunchMap`)
    (`GameplayStatics.OpenLevel` (`/Game/Blueprints/GI_CustomVehicleGameInstance.mapToLoad` (`self.gameInstance`)))))

(fn `HoveredCarChanged`
  (set `self.changingPos` false))

(fn `UpdatePickerPosition`
  (locals (getAbove :type "Float (double-precision)" :default 0.0))
  (bind (_returnvalue_x _returnvalue_y _returnvalue_z) (`KismetMathLibrary.BreakVector` (`self.K2_GetActorLocation`)))
  (bind _returnvalue_x_2 (`KismetMathLibrary.BreakVector` (`self.K2_GetActorLocation` (`|GetArrayItem` (`self.Out Actors Camera`) (`self.carPosition`)))))
  (`self.K2_SetActorLocation` (`KismetMathLibrary.MakeVector` (`KismetMathLibrary.FInterpTo` _returnvalue_x _returnvalue_x_2 (`self.Delta Seconds`) 3.0) _returnvalue_y _returnvalue_z)))

(fn `UserConstructionScript`)