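; AI-driven arcade racing car that follows a randomly chosen spline with constant throttle, steering by torque toward a look-ahead point.
; Tick simulates physics with sphere-trace spring-damper suspension at four wheels, custom gravity, anti-slide force and speed boost, then updates wheel visuals and engine audio.
; A stalled car teleports to its last checkpoint transform.
; Item, voice-line and car-select animation logic are included, while drift and handbrake logic is disconnected.
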(event `self.ReceiveBeginPlay`
  ;[1 1 1] Begin Play
  (`|ExecutionSequence`
    (:`then_0`
      (`self.InitializeConfig`)
      (`self.CustomSpline`))
    (:`then_1`
      (`self.InitializeComponentArrays`))
    (:`then_2`
      (`self.InitializePhysicsConfiguration`))
    (:`then_3`
      (bind (_direction _alpha) (`Timeline|SuspensionInitTimeline` :!via `PlayFromStart`)
        (:`Update`
          (set `self.currentSuspensionStiffness` (`KismetMathLibrary.Lerp` 0.0 (`self.suspensionStiffness`) _alpha))
          (set `self.currentSuspensionDamping` (`KismetMathLibrary.Lerp` 0.0 (`self.suspensionDamping`) _alpha)))))))

(event `InputAxis|LookUp`
  (params (AxisValue :type "Float (single-precision)"))
  (`self.AddControllerPitchInput` AxisValue))

(event `InputAxis|LookRight`
  (params (AxisValue :type "Float (single-precision)"))
  (`self.AddControllerYawInput` AxisValue))

(event `self.ReceiveTick`
  (params (DeltaSeconds :type "Float (single-precision)"))
  ;[1 1 1] Tick
  (set `self.deltaSeconds` DeltaSeconds)
  (if (`SceneComponent.IsSimulatingPhysics` (`self.VehicleCollision`) "None")
    (`|ExecutionSequence`
      (:`then_0`
        (`self.AI Throttle`))
      (:`then_1`
        (`self.AI Steering`))
      (:`then_2`
        (`self.GetCurrentMovementValues`))
      (:`then_3`
        (bind _groundwheelscount (`self.ApplySuspensionForces`))
        (`self.HandleFallingTime` _groundwheelscount))
      (:`then_4`
        (`self.UpdateCenterOfMassOffset`))
      (:`then_5`
        (`self.HandleSpeedBoost`))
      (:`then_6`
        (`self.ApplyGravityAndAntiSlidingForces`))
      (:`then_7`
        (`self.UpdateWheelsPosition`)
        (`self.UpdateWheelsRotation`)
        (`self.UpdateWheelsSteering`))
      (:`then_8`
        (`self.UpdateEngineAudio`))
      (:`then_9`
        (`KismetSystemLibrary.Delay` 0.2)
        (`self.CheckIsMove`)))))

(event `ForceResetCar`
  (bind _vehiclecollision (`self.VehicleCollision`))
  ;[1 1 1] Reset Position to Last Checkpoint
  (set `self.bCanReset` false)
  (`PrimitiveComponent.SetSimulatePhysics` _vehiclecollision false)
  (`self.K2_SetActorTransform` (`self.lastCheckPointPosition`) false true)
  (`TimelineComponent.PlayFromStart` (`self.SuspensionInitTimeline`))
  (`PrimitiveComponent.SetSimulatePhysics` _vehiclecollision true)
  (`KismetSystemLibrary.K2_SetTimer` self "ResetCarCD" 3.0))

(event `AI Throttle`
  ;[1 1 1] Throttle forward
  (if (`self.CanDrive`)
    (bind _output_get (set `self.currentThrottleAxis` 0.5))
    (if (and (>= (`KismetMathLibrary.Abs` _output_get) 0.1) (<= (`self.currentHorizontalSpeed`) (`self.maxSpeed`)) (`self.isMovingOnGround`))
      (`PrimitiveComponent.AddForce` (`self.VehicleCollision`) (* (`self.GetActorForwardVector`) (* _output_get (`self.acceleration`))) "None" true))))

(event `AI Steering`
  ;[1 1 1] Steering side
  (if (`self.CanDrive`)
    (bind _steering (`self.GetPath` (`self.Splines`)))
    (bind _output_get (set `self.currentSteeringAxis` _steering))
    (if (and (> (`self.currentHorizontalSpeed`) (`self.minSpeedToSteer`)) (>= (`KismetMathLibrary.Abs` _output_get) 0.1) (`self.isMovingOnGround`))
      (`PrimitiveComponent.AddTorqueInRadians` (`self.VehicleCollision`) (* (`self.GetActorUpVector`) (* (`self.steeringTorque`) _output_get (`KismetMathLibrary.SignOfFloat` (`self.currentMovingDirectionFake`)) (select `bool` (`self.isSpeedBoostEnabled`) :`false` 1.0 :`true` 2.0 :!type "Float (single-precision)"))) "None" true))))

(event `self.ReceivePossessed`
  (params (NewController :type "Controller Object Reference"))
  ;[1 1 1] Possess / Unpossess
  (if (not (`.bSuccess` (cast `AIController` NewController :!pure true)))
    _))

(event `SelectCarInteraction`
  (bind (_returnvalue_x _returnvalue_y _returnvalue_z) (`KismetMathLibrary.BreakVector` (`self.K2_GetActorLocation`)))
  ;[1 1 1] Select Car Anim
  (`PrimitiveComponent.SetConstraintMode` (`self.VehicleCollision`) "None")
  (bind (_direction _factor) (`Timeline|AnimateSelectCar` :!via `PlayFromStart`)
    (:`Update`
      (`self.K2_SetActorLocation` (`KismetMathLibrary.MakeVector` _returnvalue_x (+ (* _factor 700.0) (.y (.location (`self.lastCheckPointPosition`)))) _returnvalue_z)))))

(event `self.ReceiveUnpossessed`
  (params (OldController :type "Controller Object Reference"))
  ;[1 1 1] Possess / Unpossess
  (if (not (`.bSuccess` (cast `AIController` OldController :!pure true)))
    _))

(fn `ApplyGravityAndAntiSlidingForces`
  (`PrimitiveComponent.AddForce` (`self.VehicleCollision`) (* (select `bool` (< (`self.fallingTime`) 0.5) :`false` (0.0 0.0 1.0) :`true` (`self.GetActorUpVector`)) (* (`self.gravity`) -1.0)) "None" true)
  (set `self.currentSlidingSpeed` (`KismetMathLibrary.Dot_VectorVector` (`self.currentHorizontalVelocity`) (`self.GetActorRightVector`)))
  (if (and (`self.isMovingOnGround`) (> (`self.currentHorizontalSpeed`) 10.0))
    (`PrimitiveComponent.AddForce` (`self.VehicleCollision`) (* (`self.GetActorRightVector`) (* (`self.currentSlidingSpeed`) (`self.antiSlideForce`) -1.0)) "None" true)))

(fn `ApplySuspensionForces`
  (returns (groundWheelsCount :type Integer))
  (set `self.groundedWheelsNum` 0)
  (for (_array_element _array_index) (`self.localSuspensionPointsList`)
    (set `self.currentPointRelativeLocation` _array_element)
    (set `self.currentPointIndex` _array_index)
    (set `self.currentPointWorldLocation` (`KismetMathLibrary.TransformLocation` (`self.GetTransform`) (`self.currentPointRelativeLocation`)))
    (bind (_isgroundhit _ratio _applyforcelocation) (`self.PerformSuspensionRaycasts` (`self.currentPointWorldLocation`) (`self.currentPointRelativeLocation`)))
    (if _isgroundhit
      (`/Engine/EditorBlueprintResources/StandardMacros.IncrementInt` (`self.groundedWheelsNum`)
        (:`  `
          _)))
    (set `self.currentSuspensionRatio` _ratio)
    (`PrimitiveComponent.AddForceAtLocation` (`self.VehicleCollision`) (* (`self.GetActorUpVector`) (* (+ (* (`self.suspensionStiffness`) (`self.currentSuspensionRatio`)) (* (`self.suspensionDamping`) (/ (- (`self.currentSuspensionRatio`) (`|GetArrayItem` (`self.lastFrameRatios`) (`self.currentPointIndex`))) (`self.deltaSeconds`)))) (`self.massInKg`) (`self.gravity`))) _applyforcelocation "None")
    (`KismetArrayLibrary.Array_Set` (`self.lastFrameRatios`) (`self.currentPointIndex`) (`self.currentSuspensionRatio`))
    (if true
      _))
  (return (`self.groundedWheelsNum`)))

(fn `CheckIsMove`
  (if (`self.CanDrive`)
    (if (== (`self.GetVelocity`) (0.0 0.0 0.0) :`ErrorTolerance` 1.0)
      (`self.ForceResetCar`))))

(fn `CustomSpline`
  (set `self.ChooseSpline` (`KismetMathLibrary.RandomIntegerInRange` 0 (- (`KismetArrayLibrary.Array_Length` (`self.Splines`)) 1))))

(fn `GetCurrentMovementValues`
  (bind _returnvalue (`self.GetInputAxisValue`))
  (bind _vehiclecollision (`self.VehicleCollision`))
  (bind _returnvalue_2 (`KismetMathLibrary.ProjectVectorOnToPlane` (`SceneComponent.GetComponentVelocity` _vehiclecollision) (`SceneComponent.GetUpVector` _vehiclecollision)))
  (set `self.isMovingOnGround` false)
  (set `self.currentHorizontalVelocity` _returnvalue_2)
  (set `self.currentHorizontalSpeed` (`KismetMathLibrary.VSize` _returnvalue_2))
  (set `self.currentHorizontalMovementDirection` (`KismetMathLibrary.SignOfFloat` (`KismetMathLibrary.Dot_VectorVector` (`KismetMathLibrary.Normal` _returnvalue_2) (`SceneComponent.GetForwardVector` _vehiclecollision))))
  (set `self.currentMovingDirectionFake` (select `bool` (> _returnvalue 0.0) :`false` (`self.currentHorizontalMovementDirection`) :`true` _returnvalue)))

(fn `GetPath`
  (params (Splines :type "Array of /Game/Assets/Blueprint/GamePlay/BP_SplinePath Object Reference"))
  (returns (Steering :type "Float (double-precision)"))
  (bind _returnvalue (`self.K2_GetActorLocation`))
  (bind _spline (`/Game/Assets/Blueprint/GamePlay/BP_SplinePath.Spline` (`|GetArrayItem` Splines (`self.ChooseSpline`))))
  (bind (_returnvalue_roll _returnvalue_pitch _returnvalue_yaw) (`KismetMathLibrary.BreakRotator` (`KismetMathLibrary.NormalizedDeltaRotator` (`KismetMathLibrary.FindLookAtRotation` _returnvalue (`SplineComponent.FindLocationClosestToWorldLocation` _spline (+ (* (`KismetMathLibrary.Normal` (`SplineComponent.FindTangentClosestToWorldLocation` _spline _returnvalue "World") 1.0) (`self.DifferenceWithSpline`)) _returnvalue) "World")) (`self.K2_GetActorRotation`))))
  (return (`KismetMathLibrary.MapRangeClamped` _returnvalue_yaw -90.0 90.0 -4.0 4.0)))

(fn `HandleFallingTime`
  (params (groundWheelsCount :type Integer))
  (bind _output_get (set `self.isMovingOnGround` (>= groundWheelsCount (`self.minimumGroundedWheelsToMove`))))
  (set `self.fallingTime` (select `bool` _output_get :`false` (+ (`self.fallingTime`) (`self.deltaSeconds`)))))

(fn `HandleSpeedBoost`
  (if (and (`self.isSpeedBoostEnabled`) (`self.isMovingOnGround`) (<= (`self.currentHorizontalSpeed`) (`self.maxBoostSpeed`)))
    (`PrimitiveComponent.AddForce` (`self.VehicleCollision`) (* (`self.GetActorForwardVector`) (* (`self.acceleration`) (`self.speedBoostAccelerationFactor`))) "None" true)))

(fn `InitializeComponentArrays`
  (set `self.wheelMeshList` (`|MakeArray` (`self.FRWheelMesh`) (`self.FLWheelMesh`) (`self.BRWheelMesh`) (`self.BLWheelMesh`)))
  (bind _output_get (set `self.wheelSceneList` (`|MakeArray` (`self.FRWheelScene`) (`self.FLWheelScene`) (`self.BRWheelScene`) (`self.BLWheelScene`))))
  (for _array_element _output_get
    (`KismetArrayLibrary.Array_Add` (`self.localSuspensionPointsList`) (`SceneComponent.RelativeLocation` _array_element))))

(fn `InitializeConfig`
  (if (`self.shouldApplyCustomConfig`)
    (`KismetSystemLibrary.ExecuteConsoleCommand` (`KismetStringLibrary.Concat_StrStr` "t.MaxFPS " (`KismetStringLibrary.Conv_IntToString` (`self.maxFPS`))) (`GameplayStatics.GetPlayerController` 0))))

(fn `InitializePhysicsConfiguration`
  (bind _vehiclecollision (`self.VehicleCollision`))
  (`PrimitiveComponent.SetLinearDamping` _vehiclecollision (`self.linearDamping`))
  (`PrimitiveComponent.SetMassOverrideInKg` _vehiclecollision "None" (`self.massInKg`) true)
  (`PrimitiveComponent.SetAngularDamping` _vehiclecollision (`self.angularDamping`))
  (`PrimitiveComponent.SetCenterOfMass` _vehiclecollision (`self.centerOfMassOffsetWhenFalling`) "None"))

(fn `PerformSuspensionRaycasts`
  (params (suspensionPointWorldLocation :type "Vector Structure") (suspensionPointRelativeLocation :type "Vector Structure"))
  (returns (isGroundHit :type Boolean) (ratio :type "Float (double-precision)") (applyForceLocation :type "Vector Structure"))
  (bind (_returnvalue_x _returnvalue_y _returnvalue_z) (`KismetMathLibrary.BreakVector` (`BoxComponent.GetScaledBoxExtent` (`self.VehicleCollision`))))
  (bind _returnvalue (- suspensionPointWorldLocation (* (`self.GetActorUpVector`) (+ _returnvalue_z (.z suspensionPointRelativeLocation)))))
  (bind (_outhit _returnvalue_2) (`KismetSystemLibrary.SphereTraceSingleForObjects` suspensionPointWorldLocation (- suspensionPointWorldLocation (* (`self.GetActorUpVector`) (`self.suspensionHeight`))) (`self.wheelRadius`) (`self.walkableObjectTypes`) (`self.isTraceComplex`)))
  (return _returnvalue_2 (`KismetMathLibrary.FClamp` (`KismetMathLibrary.SelectFloat` (- 1.0 (/ (`KismetMathLibrary.VSize` (- (`.ImpactPoint` (`GameplayStatics.BreakHitResult` _outhit)) _returnvalue)) (`self.suspensionHeight`))) 0.0 _returnvalue_2)) _returnvalue))

(fn `ResetCarCD`
  (set `self.bCanReset` true))

(fn `SetActionsPlayer`
  (params (Action :type "/Game/Assets/Blueprint/E_ActionPlayer Enum" :default "NewEnumerator0"))
  (bind _sfx_voice (`self.SFX_Voice`))
  (bind _audioactions (`self.AudioActions`))
  (switch `/Game/Assets/Blueprint/E_ActionPlayer` Action
    (:`NewEnumerator0`
      (`AudioComponent.SetSound` _sfx_voice (`|GetArrayItem` _audioactions)))
    (:`NewEnumerator1`
      (`AudioComponent.SetSound` _sfx_voice (`|GetArrayItem` _audioactions 1)))
    (:`NewEnumerator2`
      (`AudioComponent.SetSound` _sfx_voice (`|GetArrayItem` _audioactions 2)))
    (:`NewEnumerator3`
      (`AudioComponent.SetSound` _sfx_voice (`|GetArrayItem` _audioactions 3)))
    (:`NewEnumerator4`
      (`AudioComponent.SetSound` _sfx_voice (`|GetArrayItem` _audioactions 4))))
  (`AudioComponent.Play` _sfx_voice 0.0))

(fn `SpeedBoostEnd`
  (if (`KismetSystemLibrary.K2_IsTimerActiveHandle` (`self.speedBoostTimerHandle`))
    (`KismetSystemLibrary.K2_ClearAndInvalidateTimerHandle` (`self.speedBoostTimerHandle`)))
  (set `self.isSpeedBoostEnabled` false))

(fn `SpeedBoostStart`
  (params (speedBoostFactor :type "Float (double-precision)" :default 2.0) (autoStop :type Boolean :default true) (speedBoostDuration :type "Float (double-precision)" :default 2.0))
  (set `self.isSpeedBoostEnabled` true)
  (set `self.speedBoostAccelerationFactor` speedBoostFactor)
  (if autoStop
    (bind _returnvalue (`KismetSystemLibrary.K2_SetTimer` null "SpeedBoostEnd" (`KismetMathLibrary.FMax` 0.0 speedBoostDuration)))
    (set `self.speedBoostTimerHandle` _returnvalue)))

(fn `UpdateCenterOfMassOffset`
  (`PrimitiveComponent.SetCenterOfMass` (`self.VehicleCollision`) (select `bool` (> (`self.fallingTime`) 1.0) :`false` (`self.centerOfMassOffsetWhenMoving`) :`true` (`self.centerOfMassOffsetWhenFalling`)) "None"))

(fn `UpdateEngineAudio`
  (`AudioComponent.SetFloatParameter` (`self.EngineAudio`) "Speed" (`self.currentHorizontalSpeed`)))

(fn `UpdateWheelsPosition`
  (for (_array_element _array_index) (`self.wheelSceneList`)
    (bind (_output_x _output_y _output_z) (`KismetMathLibrary.BreakVector` (`|GetArrayItem` (`self.localSuspensionPointsList`) _array_index)))
    (`SceneComponent.K2_SetRelativeLocation` _array_element (`KismetMathLibrary.VLerp` (`SceneComponent.RelativeLocation` _array_element) (`KismetMathLibrary.MakeVector` _output_x _output_y (+ _output_z (* (- 1.0 (`|GetArrayItem` (`self.lastFrameRatios`) _array_index)) (`self.suspensionHeight`) -1.0) (`self.wheelRadius`))) (`KismetMathLibrary.FClamp` (* (`self.deltaSeconds`) 10.0))) false false)))

(fn `UpdateWheelsRotation`
  (for _array_element (`self.wheelMeshList`)
    (`SceneComponent.K2_AddLocalRotation` _array_element (`KismetMathLibrary.MakeRotator` 0.0 (* (`self.currentHorizontalSpeed`) (`self.currentHorizontalMovementDirection`) (`KismetMathLibrary.SignOfFloat` (`KismetMathLibrary.Dot_VectorVector` (`SceneComponent.GetRightVector` _array_element) (`SceneComponent.GetRightVector` (`self.VehicleCollision`)))) (`KismetMathLibrary.GetPI`) (`GameplayStatics.GetWorldDeltaSeconds`) -1.0 0.1)) false false)))

(fn `UpdateWheelsSteering`
  (for _index (range 2)
    (bind _output (`|GetArrayItem` (`self.wheelSceneList`) _index))
    (bind (_relativerotation_roll _relativerotation_pitch _relativerotation_yaw) (`KismetMathLibrary.BreakRotator` (`SceneComponent.RelativeRotation` _output)))
    (`SceneComponent.K2_SetRelativeRotation` _output (`KismetMathLibrary.MakeRotator` 0.0 0.0 (`KismetMathLibrary.Lerp` _relativerotation_yaw (* (`self.GetInputAxisValue`) (`self.maxSteerAngle`)) (* (`self.deltaSeconds`) 15.0))) false false)))

(fn `UseItem`
  (switch `/Game/Blueprints/Gameplay/E_ItemTypes` (`self.currentItemType`)
    (:`NewEnumerator0`
      (`self.SpeedBoostStart` 1.2 true 1.0)
      (set `self.currentItemType` "NewEnumerator2" :!label _label))
    (:`NewEnumerator1`
      (bind _outactors (`GameplayStatics.GetAllActorsOfClass` "BP_CustomArcadeVehicle_AI_C"))
      (for _array_element _outactors
        (if (!= _array_element self)
          (`self.SpeedBoostStart` _array_element 0.8 true 1.0)
          (goto _label))))))

(fn `UserConstructionScript`
  (set `self.lastCheckPointPosition` (`self.GetTransform`))
  (set `self.bCanReset` true))