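; Game mode for the racing game that spawns each local player's chosen vehicle and applies the selected race mode.
; On BeginPlay it reads the vehicles and mode from the game instance, replaces one BP_RaceSpawner per vehicle with that vehicle, and possesses it, creating extra local players as needed.
; LoadGameMode then adjusts the match: Time Attack removes items and hides item and position HUD, while Survie hides only position.
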(event `self.ReceiveBeginPlay`
  (bind _asgi_custom_vehicle_game_instance (cast `/Game/Blueprints/GI_CustomVehicleGameInstance` (`GameplayStatics.GetGameInstance`)))
  (set `self.GameMode` (`/Game/Blueprints/GI_CustomVehicleGameInstance.GameModeToLoad` _asgi_custom_vehicle_game_instance))
  (bind _outactors (`GameplayStatics.GetAllActorsOfClass` "/Game/Blueprints/Gameplay/BP_RaceSpawner.BP_RaceSpawner_C"))
  (set `self.Out Actors` _outactors)
  (for (_array_element _array_index) (`/Game/Blueprints/GI_CustomVehicleGameInstance.vehicles` _asgi_custom_vehicle_game_instance)
    (for _array_element_2 (`self.Out Actors`)
      (`KismetSystemLibrary.PrintString` (`KismetSystemLibrary.GetClassDisplayName` _array_element))
      (if (> _array_index 0)
        (`GameplayStatics.CreatePlayer` _array_index))
      (`GameplayStatics.GetActorOfClass` "/Game/Blueprints/Cars/CustomArcadeVehicle/BP_CustomArcadeVehicle.BP_CustomArcadeVehicle_C")
      (bind _returnvalue (`|SpawnActorFromClass` _array_element (`self.GetTransform` _array_element_2) "Undefined" "OverrideRootScale" null _array_index (`KismetTextLibrary.Conv_StringToText` (`KismetStringLibrary.Concat_StrStr` "Racer " (`KismetStringLibrary.Conv_IntToString` (+ _array_index 1)))) null))
      (`self.K2_DestroyActor` _array_element_2)
      (bind _returnvalue_2 (`GameplayStatics.GetPlayerControllerFromID` _array_index))
      (`Controller.UnPossess` _returnvalue_2)
      (`Controller.Possess` _returnvalue_2 _returnvalue)
      (`KismetArrayLibrary.Array_RemoveItem` (`self.Out Actors`) _array_element_2)
      (break)))
  (`self.Load GameMode`))

(event `Load GameMode`
  (switch `name` (`self.GameMode`)
    (:`TimeAttack`
      (bind _outactors (`GameplayStatics.GetAllActorsOfClass` "/Game/Blueprints/Gameplay/BP_Item.BP_Item_C"))
      (for _array_element _outactors
        (`self.K2_DestroyActor` _array_element))
      (bind _outactors_2 (`GameplayStatics.GetAllActorsOfClass` "/Game/Blueprints/Cars/CustomArcadeVehicle/BP_CustomArcadeVehicle.BP_CustomArcadeVehicle_C"))
      (for _array_element_2 _outactors_2
        (bind _ingamehud (`/Game/Blueprints/Cars/CustomArcadeVehicle/BP_CustomArcadeVehicle.inGameHUD` _array_element_2))
        (`/Game/UI/WBP_InGameHUD.Disable Object Interface` _ingamehud)
        (`/Game/UI/WBP_InGameHUD.Disable Pos Interface` _ingamehud)))
    (:`Survie`
      (bind _outactors_3 (`GameplayStatics.GetAllActorsOfClass` "/Game/Blueprints/Cars/CustomArcadeVehicle/BP_CustomArcadeVehicle.BP_CustomArcadeVehicle_C"))
      (for _array_element_3 _outactors_3
        (`/Game/UI/WBP_InGameHUD.Disable Pos Interface` (`/Game/Blueprints/Cars/CustomArcadeVehicle/BP_CustomArcadeVehicle.inGameHUD` _array_element_3))))))

(fn `UserConstructionScript`)