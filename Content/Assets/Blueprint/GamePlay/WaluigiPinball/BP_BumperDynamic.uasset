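; BP_BumperDynamic is a moving bumper for the Waluigi Pinball level that knocks arcade vehicles backward on contact.
; Each tick, transform composition swings the mesh around PointPivot by DeltaRotation, counter-rotates it, then adds a fixed yaw step independent of frame time.
; On hit, it overrides the vehicle's velocity along its reversed forward vector, adds a matching velocity-change impulse and sets the player's action state.
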(event `self.ReceiveTick`
  (params (DeltaSeconds :type "Float (single-precision)"))
  (bind _staticmesh (`self.StaticMesh`))
  (bind _staticmesh_2 (`self.StaticMesh`))
  (bind (_relativerotation_roll _relativerotation_pitch _relativerotation_yaw) (`KismetMathLibrary.BreakRotator` (`SceneComponent.RelativeRotation` _staticmesh)))
  (bind _returnvalue (`KismetMathLibrary.MakeTransform` (`SceneComponent.K2_GetComponentLocation` (`self.PointPivot`)) (`SceneComponent.K2_GetComponentRotation` _staticmesh_2)))
  (set `self.Delta Seconds` DeltaSeconds)
  (`SceneComponent.K2_SetWorldTransform` (`self.StaticMesh`) (`KismetMathLibrary.ComposeTransforms` (`KismetMathLibrary.MakeTransform` (0.0 0.0 0.0) (`KismetMathLibrary.NegateRotator` (`self.Delta Rotation`))) (`KismetMathLibrary.ComposeTransforms` (`KismetMathLibrary.ComposeTransforms` (`SceneComponent.K2_GetComponentToWorld` _staticmesh_2) (`KismetMathLibrary.InvertTransform` _returnvalue)) (`KismetMathLibrary.ComposeTransforms` (`KismetMathLibrary.MakeTransform` (0.0 0.0 0.0) (`self.Delta Rotation`)) _returnvalue))) false false)
  (`SceneComponent.K2_SetRelativeRotation` _staticmesh (`KismetMathLibrary.MakeRotator` 0.0 0.0 (+ _relativerotation_yaw 1.0)) false false))

(event `self.StaticMesh.OnComponentHit`
  (params (HitComponent :type "PrimitiveComponent Object Reference") (OtherActor :type "Actor Object Reference") (OtherComp :type "PrimitiveComponent Object Reference") (NormalImpulse :type "Vector Structure") (Hit :type "HitResult Structure (by ref)"))
  (bind _asbp_custom_arcade_vehicle (cast `/Game/Blueprints/Cars/CustomArcadeVehicle/BP_CustomArcadeVehicle` OtherActor))
  (bind _vehiclecollision (`/Game/Blueprints/Cars/CustomArcadeVehicle/BP_CustomArcadeVehicle.VehicleCollision` _asbp_custom_arcade_vehicle))
  (bind _returnvalue (* (`self.GetActorForwardVector` _asbp_custom_arcade_vehicle) -1200.0))
  (`PrimitiveComponent.SetPhysicsLinearVelocity` _vehiclecollision _returnvalue false "None")
  (`PrimitiveComponent.AddImpulse` _vehiclecollision _returnvalue "None" true)
  (`/Game/Blueprints/Cars/CustomArcadeVehicle/BP_CustomArcadeVehicle.SetActionsPlayer` _asbp_custom_arcade_vehicle "NewEnumerator1"))

(fn `UserConstructionScript`)