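; Pinball flipper obstacle for the Waluigi Pinball level that randomly swings open or closed and knocks back vehicles that hit it.
; A self-restarting one-second timer gives an even chance of toggling the open state.
; Tick smoothly interpolates rotation toward one of four rotators chosen by side and open state.
; Mesh hits throw arcade vehicles backward via velocity and impulse, then after a short delay apply damage and set their action state.
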(event `TryOpen`
  ;[1 0.8648 0.1491] Random Open
  (if (`KismetMathLibrary.RandomBoolWithWeight` 0.5)
    (if (`self.IsOpen?`)
      (set `self.IsOpen?` false)
      (else
        (set `self.IsOpen?` true))))
  (`KismetSystemLibrary.K2_SetTimerDelegate` (delegate `TryOpen`) 1.0))

(event `self.ReceiveBeginPlay`
  ;[0.3021 0.2916 0.2187] Init
  (`self.TryOpen`))

(event `self.ReceiveTick`
  (params (DeltaSeconds :type "Float (single-precision)"))
  ;[0.2532 1 0.2549] Animate Flipper
  (set `self.Delta Seconds` DeltaSeconds)
  (`self.K2_SetActorRotation` (`KismetMathLibrary.RInterpTo` (`self.K2_GetActorRotation`) (`KismetMathLibrary.SelectRotator` (`KismetMathLibrary.SelectRotator` (`self.SideTrueTrueA`) (`self.SideTrueFalseB`) (`self.IsOpen?`)) (`KismetMathLibrary.SelectRotator` (`self.SideFalseTrueA`) (`self.SideFalseFalseB`) (`self.IsOpen?`)) (`self.Side?`)) (`self.Delta Seconds`) 5.0)))

(event `self.StaticMesh.OnComponentHit`
  (params (HitComponent :type "PrimitiveComponent Object Reference") (OtherActor :type "Actor Object Reference") (OtherComp :type "PrimitiveComponent Object Reference") (NormalImpulse :type "Vector Structure") (Hit :type "HitResult Structure (by ref)"))
  ;[0.2165 0.5325 1] Event Trigger
  (bind _asbp_custom_arcade_vehicle (cast `/Game/Blueprints/Cars/CustomArcadeVehicle/BP_CustomArcadeVehicle` OtherActor))
  (bind _vehiclecollision (`/Game/Blueprints/Cars/CustomArcadeVehicle/BP_CustomArcadeVehicle.VehicleCollision` _asbp_custom_arcade_vehicle))
  (bind _returnvalue (* (`self.GetActorForwardVector` _asbp_custom_arcade_vehicle) -1200.0))
  (`PrimitiveComponent.SetPhysicsLinearVelocity` _vehiclecollision _returnvalue false "None")
  (`PrimitiveComponent.AddImpulse` _vehiclecollision _returnvalue "None" true)
  (`KismetSystemLibrary.Delay` 0.25)
  (`GameplayStatics.ApplyDamage` _asbp_custom_arcade_vehicle 1.0)
  (`/Game/Blueprints/Cars/CustomArcadeVehicle/BP_CustomArcadeVehicle.SetActionsPlayer` _asbp_custom_arcade_vehicle "NewEnumerator1"))

(fn `UserConstructionScript`)