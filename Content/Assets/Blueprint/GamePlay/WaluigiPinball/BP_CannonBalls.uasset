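; BP_CannonBalls is a Waluigi Pinball hazard that travels along a spline and knocks back vehicles it hits.
; On BeginPlay it uses its assigned BP_SplinePath or finds one, then plays a timeline at a rate set by CircuitTimeSeconds.
; The timeline drives location and rotation by spline distance, forcing a fixed scale.
; Hitting a BP_CustomArcadeVehicle overrides its velocity backward, adds a backward impulse, then applies damage after a short delay.
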(event `self.ReceiveBeginPlay`
  (`/Engine/EditorBlueprintResources/StandardMacros.IsValid` (`self.SplinePath`)
    (:`Is Valid`
      _)
    (:`Is Not Valid`
      (bind _returnvalue (`GameplayStatics.GetActorOfClass` "/Game/Assets/Blueprint/GamePlay/WaluigiPinball/BP_SplinePath.BP_SplinePath_C"))
      (set `self.SplinePath` _returnvalue)))
  (`self.Move Object`))

(event `Move Object`
  (bind _spline (`/Game/Assets/Blueprint/GamePlay/WaluigiPinball/BP_SplinePath.Spline` (`self.SplinePath`)))
  (`TimelineComponent.SetPlayRate` (`self.Moving Object`) (/ 1.0 (`self.Circuit Time (seconds)`)))
  (bind (_direction _move_track) (`Timeline|Moving Object`)
    (:`Update`
      (bind _returnvalue (`KismetMathLibrary.Lerp` 0.0 (`SplineComponent.GetSplineLength` (`/Game/Assets/Blueprint/GamePlay/WaluigiPinball/BP_SplinePath.Spline` (`self.SplinePath`))) _move_track))
      (`self.K2_SetActorTransform` (`KismetMathLibrary.MakeTransform` (`SplineComponent.GetLocationAtDistanceAlongSpline` _spline _returnvalue "World") (`SplineComponent.GetRotationAtDistanceAlongSpline` _spline _returnvalue "World") (3.0 3.0 3.0))))))

(event `self.CannonBalls.OnComponentHit`
  (params (HitComponent :type "PrimitiveComponent Object Reference") (OtherActor :type "Actor Object Reference") (OtherComp :type "PrimitiveComponent Object Reference") (NormalImpulse :type "Vector Structure") (Hit :type "HitResult Structure (by ref)"))
  (bind _asbp_custom_arcade_vehicle (cast `/Game/Blueprints/Cars/CustomArcadeVehicle/BP_CustomArcadeVehicle` OtherActor))
  (bind _vehiclecollision (`/Game/Blueprints/Cars/CustomArcadeVehicle/BP_CustomArcadeVehicle.VehicleCollision` _asbp_custom_arcade_vehicle))
  (bind _returnvalue (* (`self.GetActorForwardVector` _asbp_custom_arcade_vehicle) -1200.0))
  (`PrimitiveComponent.SetPhysicsLinearVelocity` _vehiclecollision _returnvalue false "None")
  (`PrimitiveComponent.AddImpulse` _vehiclecollision _returnvalue "None" true)
  (`KismetSystemLibrary.Delay` 0.25)
  (`GameplayStatics.ApplyDamage` _asbp_custom_arcade_vehicle 1.0))

(fn `UserConstructionScript`)