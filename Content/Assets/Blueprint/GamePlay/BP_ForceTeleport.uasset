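; BP_ForceTeleport is a trigger actor that pulls overlapping BP_CustomArcadeVehicle actors to its TeleportPoint.
; Trigger overlap adds each vehicle uniquely to a target array.
; Every Tick interpolates queued vehicles' location and rotation toward the point without sweep or physics teleport, so movement is a glide.
; A vehicle leaves the array once within a loose distance tolerance of the point, ending that frame's loop.
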(event `TeleportVehicle`
  (bind _returnvalue (`SceneComponent.K2_GetComponentLocation` (`self.TeleportPoint`)))
  (if (!= (`KismetArrayLibrary.Array_Length` (`self.ArrayInTarget`)) 0)
    (for _array_element (`self.ArrayInTarget`)
      (bind _returnvalue_2 (`self.K2_GetActorLocation` _array_element))
      (`self.K2_SetActorLocation` _array_element (`KismetMathLibrary.VInterpTo` _returnvalue_2 _returnvalue (`self.Delta Seconds`) (`self.Interp Speed Location`)) false false)
      (`self.K2_SetActorRotation` _array_element (`KismetMathLibrary.RInterpTo` (`self.K2_GetActorRotation` _array_element) (`SceneComponent.K2_GetComponentRotation` (`self.TeleportPoint`)) (`self.Delta Seconds`) (`self.Interp Speed Rotation`)) false)
      (if (== _returnvalue_2 _returnvalue :`ErrorTolerance` 1000.0)
        (bind _returnvalue_3 (`KismetArrayLibrary.Array_RemoveItem` (`self.ArrayInTarget`) _array_element))
        (if _returnvalue_3
          (break))))))

(event `self.ReceiveTick`
  (params (DeltaSeconds :type "Float (single-precision)"))
  (set `self.Delta Seconds` DeltaSeconds)
  (`self.TeleportVehicle`))

(event `self.Trigger.OnComponentBeginOverlap`
  (params (OverlappedComponent :type "PrimitiveComponent Object Reference") (OtherActor :type "Actor Object Reference") (OtherComp :type "PrimitiveComponent Object Reference") (OtherBodyIndex :type Integer) (bFromSweep :type Boolean) (SweepResult :type "HitResult Structure (by ref)"))
  (bind _asbp_custom_arcade_vehicle (cast `/Game/Blueprints/Cars/CustomArcadeVehicle/BP_CustomArcadeVehicle` OtherActor))
  (`self.AddVehicle` _asbp_custom_arcade_vehicle))

(event `AddVehicle`
  (params (Actor :type "Actor Object Reference"))
  (`KismetArrayLibrary.Array_AddUnique` (`self.ArrayInTarget`) Actor))

(fn `UserConstructionScript`)