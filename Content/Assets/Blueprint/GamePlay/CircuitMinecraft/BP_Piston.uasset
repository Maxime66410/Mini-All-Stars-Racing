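; Minecraft-circuit piston obstacle that randomly extends or retracts and knocks arcade vehicles away.
; A self-rearming one-second timer gives a 50% chance to flip the open state, swapping the torch material and sound.
; Tick eases the arm toward the matching position with VInterpTo.
; An arm hit on a custom arcade vehicle launches it along the arm's up vector, sets its player action and calls BallonTakeDown.
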(event `TryOpen`
  (bind _torch (`self.Torch`))
  (bind _materialstorch (`self.MaterialsTorch`))
  (bind _audio (`self.Audio`))
  (bind _audiofiles (`self.AudioFiles`))
  ;[1 0.8648 0.1491] Random Open
  (if (`KismetMathLibrary.RandomBoolWithWeight` 0.5)
    (if (`self.IsOpen?`)
      (set `self.IsOpen?` false)
      (`PrimitiveComponent.SetMaterial` _torch 0 (`|GetArrayItem` _materialstorch))
      (`AudioComponent.SetSound` _audio (`|GetArrayItem` _audiofiles))
      (else
        (set `self.IsOpen?` true)
        (`PrimitiveComponent.SetMaterial` _torch 0 (`|GetArrayItem` _materialstorch 1))
        (`AudioComponent.SetSound` _audio (`|GetArrayItem` _audiofiles 1))))
    (`AudioComponent.Play` _audio 0.0))
  (`KismetSystemLibrary.K2_SetTimerDelegate` (delegate `TryOpen`) 1.0))

(event `self.ReceiveBeginPlay`
  ;[0.3021 0.2916 0.2187] Init
  (`self.TryOpen`))

(event `self.ReceiveTick`
  (params (DeltaSeconds :type "Float (single-precision)"))
  (bind _pistonarm (`self.PistonArm`))
  ;[0.2532 1 0.2549] Animate Flipper
  (set `self.Delta Seconds` DeltaSeconds)
  (`SceneComponent.K2_SetRelativeLocation` _pistonarm (`KismetMathLibrary.VInterpTo` (`SceneComponent.RelativeLocation` _pistonarm) (select `bool` (`self.IsOpen?`) :`false` (0.0 0.0 -69.090912) :!type "Vector Structure") (`self.Delta Seconds`) 10.0) false false))

(event `self.PistonArm.OnComponentHit`
  (params (HitComponent :type "PrimitiveComponent Object Reference") (OtherActor :type "Actor Object Reference") (OtherComp :type "PrimitiveComponent Object Reference") (NormalImpulse :type "Vector Structure") (Hit :type "HitResult Structure (by ref)"))
  (bind _returnvalue (* (`SceneComponent.GetUpVector` (`self.PistonArm`)) 500.0))
  ;[1 0.8261 0.1073] Trigger Hit
  (bind _asbp_custom_arcade_vehicle (cast `/Game/Blueprints/Cars/CustomArcadeVehicle/BP_CustomArcadeVehicle` OtherActor))
  (bind _vehiclecollision (`/Game/Blueprints/Cars/CustomArcadeVehicle/BP_CustomArcadeVehicle.VehicleCollision` _asbp_custom_arcade_vehicle))
  (`PrimitiveComponent.SetPhysicsLinearVelocity` _vehiclecollision _returnvalue false "None")
  (`PrimitiveComponent.AddImpulse` _vehiclecollision _returnvalue "None" true)
  (`/Game/Blueprints/Cars/CustomArcadeVehicle/BP_CustomArcadeVehicle.SetActionsPlayer` _asbp_custom_arcade_vehicle "NewEnumerator1")
  (`/Game/Blueprints/Cars/CustomArcadeVehicle/BP_CustomArcadeVehicle.BallonTakeDown` _asbp_custom_arcade_vehicle))

(fn `UserConstructionScript`)