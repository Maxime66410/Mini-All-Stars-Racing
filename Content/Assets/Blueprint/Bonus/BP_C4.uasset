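; C4 bonus actor: a beeping explosive that detonates on a countdown or when a vehicle hits it.
; One-second looping-by-retrigger timers drive the beep and the countdown, which advances only after SetExplode arms it.
; Player or AI vehicle hits detonate it immediately, even unarmed, and call SetActionsPlayer.
; Detonation hides the mesh, ignores collision, spawns effects, applies radial damage and destroys the actor after a delay.
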(event `BeepPlay`
  ;[1 1 1] Beep Play
  (if (not (`self.isExplode`))
    (`AudioComponent.Play` (`self.Beep`) 0.0)
    (`KismetSystemLibrary.K2_SetTimerDelegate` (delegate `BeepPlay`) 1.0)))

(event `TimerExplode`
  (bind _explode (`self.Explode`))
  (bind _returnvalue (`SceneComponent.K2_GetComponentLocation` (`self.w_c4`)))
  ;[1 1 1] Timer Explosion Event
  (if (`self.CanExplode?`)
    (`/Engine/EditorBlueprintResources/StandardMacros.IncrementInt` (`self.CountExplode`)
      (:`  `
        (if (== (`self.CountExplode`) 5)
          (set `self.isExplode` true :!label _label)
          (`AudioComponent.SetSound` _explode "/Game/Assets/Audio/SoundEffects/Bonus/C4/c4_explode1.c4_explode1")
          (`AudioComponent.Play` _explode 0.0)
          (`SceneComponent.SetVisibility` (`self.w_c4`) false false)
          (`PrimitiveComponent.SetCollisionResponseToAllChannels` (`self.Box`) "ECR_Ignore")
          (`GameplayStatics.SpawnEmitterAtLocation` "/Game/StarterContent/Particles/P_Explosion.P_Explosion" _returnvalue (struct) (10.0 10.0 10.0))
          (`GameplayStatics.ApplyRadialDamage` :`BaseDamage` 1.0 :`Origin` _returnvalue :`DamageRadius` 650.0 :`DamageCauser` null :`InstigatedByController` null)
          (`KismetSystemLibrary.Delay` 4.0)
          (`self.K2_DestroyActor`)
          (else
            (`KismetSystemLibrary.K2_SetTimerDelegate` (delegate `TimerExplode`) 1.0 :!label _label_2)))))
    (else
      (goto _label_2))))

(event `AutoExplode`
  ;[1 1 1] If Player hit
  (goto _label))

(event `self.ReceiveBeginPlay`
  ;[1 1 1] Auto Play
  (`self.BeepPlay`)
  (`self.TimerExplode`))

(event `SetExplode`
  (bind _pose (`self.Pose`))
  ;[1 1 1] Setup Explode
  (set `self.CanExplode?` true)
  (`AudioComponent.SetSound` _pose "/Game/Assets/Audio/SoundEffects/Bonus/C4/c4_plant.c4_plant")
  (`AudioComponent.Play` _pose 0.0))

(event `self.Box.OnComponentHit`
  (params (HitComponent :type "PrimitiveComponent Object Reference") (OtherActor :type "Actor Object Reference") (OtherComp :type "PrimitiveComponent Object Reference") (NormalImpulse :type "Vector Structure") (Hit :type "HitResult Structure (by ref)"))
  ;[1 1 1] Auto Explode
  (bind _asbp_custom_arcade_vehicle (cast `/Game/Blueprints/Cars/CustomArcadeVehicle/BP_CustomArcadeVehicle` OtherActor)
    (:`then`
      _)
    (:`CastFailed`
      (cast `/Game/Assets/Blueprint/AI/BP_CustomArcadeVehicle_AI` OtherActor)))
  (`self.AutoExplode`)
  (`/Game/Blueprints/Cars/CustomArcadeVehicle/BP_CustomArcadeVehicle.SetActionsPlayer` _asbp_custom_arcade_vehicle "NewEnumerator1"))

(fn `UserConstructionScript`)