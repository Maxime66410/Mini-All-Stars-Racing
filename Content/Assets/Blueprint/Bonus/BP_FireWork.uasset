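; Firework rocket bonus actor that, once launched, flies until it touches something and explodes.
; SetCanMove starts the flight and launch sound, and Tick moves it backward along its forward vector by a fixed, frame-rate-dependent step without sweeping.
; A Box hit or overlap disables collision, removes the rocket and trail components, spawns Niagara and sound effects, applies radial damage, then destroys the actor after a delay.
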(event `self.ReceiveTick`
  (params (DeltaSeconds :type "Float (single-precision)"))
  ;[1 1 1] Infinite forward
  (if (`self.IsLaunch`)
    (if (not (`self.IsExplode`))
      (`self.K2_SetActorLocation` (+ (`self.K2_GetActorLocation`) (* (`self.GetActorForwardVector`) -25.0))))))

(event `self.Box.OnComponentHit`
  (params (HitComponent :type "PrimitiveComponent Object Reference") (OtherActor :type "Actor Object Reference") (OtherComp :type "PrimitiveComponent Object Reference") (NormalImpulse :type "Vector Structure") (Hit :type "HitResult Structure (by ref)"))
  (bind _explode (`self.Explode`))
  (bind _returnvalue (`SceneComponent.K2_GetComponentLocation` (`self.Box`)))
  ;[1 1 1] Explode Firework
  (if (`self.IsLaunch`) :!label _label
    (set `self.IsExplode` true)
    (`AudioComponent.SetSound` _explode "/Game/Assets/Audio/SoundEffects/Bonus/FireWork/FireWork_Explode.FireWork_Explode")
    (`AudioComponent.Play` _explode 0.0)
    (`PrimitiveComponent.SetCollisionResponseToAllChannels` (`self.Box`) "ECR_Ignore")
    (`ActorComponent.K2_DestroyComponent` (`self.Niagara`))
    (`ActorComponent.K2_DestroyComponent` (`self.FireworkRocket`))
    (`NiagaraFunctionLibrary.SpawnSystemAtLocation` "/Game/Assets/Particle/FireWork/NG_FireWorkExplode.NG_FireWorkExplode" _returnvalue (struct) (3.0 3.0 3.0))
    (`GameplayStatics.ApplyRadialDamage` :`BaseDamage` 1.0 :`Origin` _returnvalue :`DamageRadius` 450.0 :`DamageCauser` null :`InstigatedByController` null)
    (`KismetSystemLibrary.Delay` 3.0)
    (`self.K2_DestroyActor`)))

(event `self.Box.OnComponentBeginOverlap`
  (params (OverlappedComponent :type "PrimitiveComponent Object Reference") (OtherActor :type "Actor Object Reference") (OtherComp :type "PrimitiveComponent Object Reference") (OtherBodyIndex :type Integer) (bFromSweep :type Boolean) (SweepResult :type "HitResult Structure (by ref)"))
  ;[1 1 1] Explode Firework
  (goto _label))

(event `SetCanMove`
  (bind _fire (`self.Fire`))
  ;[1 1 1] Set Can Move
  (set `self.IsLaunch` true)
  (`AudioComponent.SetSound` _fire "/Game/Assets/Audio/Player/Steve/launch1.launch1")
  (`AudioComponent.Play` _fire 0.0))

(fn `UserConstructionScript`)